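; BP_Test is a test actor Blueprint that prints the sum of two integers when play begins.
; BeginPlay calls the AddNumber function, which returns the sum of its two inputs, and prints the result as a string.
; Overlap, Tick and the construction script are empty, and leftover unconnected nodes for doubling FirstNumber and printing never run.
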(event `self.ReceiveBeginPlay`
  (bind _c (`self.AddNumber` 2 3))
  (`KismetSystemLibrary.PrintString` (`KismetStringLibrary.Conv_IntToString` _c)))

(event `self.ReceiveTick`
  (params (DeltaSeconds :type "Float (single-precision)")))

(fn `AddNumber`
  (params (A :type Integer) (B :type Integer))
  (returns (C :type Integer))
  (return (+ A B)))

(fn `UserConstructionScript`)